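; Firebolt spell gameplay ability that fires a spell toward the point under the mouse.
; On activation it takes the trace end of the mouse target data, turns the avatar toward it through CombatInterface, and plays the finger-blast montage.
; Two chained montage gameplay events drive the spell: the first calls InitSpellAbility, the second ActivateSpellAbility, both with that location.
; The ability ends after a short delay following the fired event.
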(event `self.K2_ActivateAbility`
  (bind (_asynctaskproxy _data) (`TargetDataUnderMouse.CreateTargetDataUnderMouse`)
    (:`then`
      (bind _output_get (set `self.SpawnLocation` (`.TraceEnd` (`GameplayStatics.BreakHitResult` (`AbilitySystemBlueprintLibrary.GetHitResultFromTargetData` _data)))))
      (bind _ascombat_interface (cast `CombatInterface` (`self.GetAvatarActorFromActorInfo`)))
      (`CombatInterface.SetTargetFaceDirection` _ascombat_interface _output_get)
      (`AbilityTask_PlayMontageAndWait.CreatePlayMontageAndWaitProxy` "None" "/Game/Blueprints/Characters/Player/Harry/Animation/Montage/AM_Harry_Finger_Blast.AM_Harry_Finger_Blast" 1.0 "1"
        (:`then`
          (`AbilityTask_WaitGameplayEvent.WaitGameplayEvent` (struct :`TagName` "Event.Montage.Firebolt") null
            (:`EventReceived`
              (`self.InitSpellAbility` (`self.SpawnLocation`))
              (`AbilityTask_WaitGameplayEvent.WaitGameplayEvent` (struct :`TagName` "Event.Montage.Firebolt_Fired") null
                (:`EventReceived`
                  (`self.ActivateSpellAbility` (`self.SpawnLocation`))
                  (`KismetSystemLibrary.Delay` 1.0)
                  (`self.K2_EndAbility`))))))))))